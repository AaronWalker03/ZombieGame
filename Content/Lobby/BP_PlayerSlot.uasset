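; BP_PlayerSlot is a lobby slot actor that shows a character standing in for the player assigned to it.
; AddPlayer stores the controller, replaces any existing character with a new BP_FirstPersonCharacter at the Arrow's transform, and raises it by the capsule half height above the arrow.
; RemovePlayer clears the controller and destroys the spawned character.
; The spawned character is never possessed here.
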(event Custom|AddPlayer
  (params (PlayerController :type Player%20Controller%20Object%20Reference))
  (bind _arrow (Variables|Default|GetArrow))
  (bind _returnvalue (Transformation|GetWorldTransform _arrow))
  (Variables|Default|SetPlayerController PlayerController)
  (bind _selectedcharacter (Variables|Default|GetSelectedCharacter)
    (:then
      (Actor|DestroyActor _selectedcharacter))
    (:else
      _))
  (bind _returnvalue_2 (Game|SpawnActorfromClass "/Game/FirstPerson/Blueprints/BP_FirstPersonCharacter.BP_FirstPersonCharacter_C" (Transformation|GetWorldTransform (Variables|Default|GetArrow)) "AlwaysSpawn" "MultiplyWithRoot" 0 0))
  (bind _output_get (Variables|Default|SetSelectedCharacter _returnvalue_2))
  (Transformation|SetActorTransform _output_get (Math|Transform|MakeTransform (Math|Vector|MakeVector (.x (.location _returnvalue)) (.y (.location _returnvalue)) (+ (Components|Capsule|GetScaledCapsuleHalfHeight (Variables|/Script/Engine.Character|GetCapsuleComponent _returnvalue_2)) (.z (.location _returnvalue)))) (.rotation _returnvalue) (.scale _returnvalue))))

(event Custom|RemovePlayer
  (Variables|Default|SetPlayerController 0)
  (bind _selectedcharacter (Variables|Default|GetSelectedCharacter)
    (:then
      (Actor|DestroyActor _selectedcharacter)
      (Variables|Default|SetSelectedCharacter 0))
    (:else)))

(fn ConstructionScript)