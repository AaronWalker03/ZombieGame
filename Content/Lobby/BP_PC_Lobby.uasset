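; Lobby player controller that sets up the local player's session UI and registers the player's info with the lobby game mode.
; On BeginPlay, the local controller creates a session manager widget, adds the lobby UI to the viewport, and enables the cursor with game-and-UI input.
; A "ROS" (run-on-server) event passes the controller to BP_LobbyGameMode, called at startup and by UpdatePlayerInfo after a short delay.
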(event Custom|Update%20Player%20Info
  (Utilities|FlowControl|Delay 0.1)
  (CallFunction|ROSUpdatePlayerInfo))

(event Custom|ROS_Update%20Player%20Info
  (bind _asbp_lobby_game_mode (Utilities|Casting|CastToBP_LobbyGameMode (Game|GetGameMode)))
  (Default|UpdatePlayerInfo _asbp_lobby_game_mode self))

(event EventBeginPlay
  (if (Pawn|IsLocalPlayerController)
    (UserInterface|CreateWidget "/Game/UI/BPs/WB_SessionManager.WB_SessionManager_C")
    (bind _output_get (Variables|Default|SetLobby%20UI 0))
    (UserInterface|Viewport|AddtoViewport _output_get 0)
    (Variables|Default|SetbShowMouseCursor true)
    (Input|SetInputModeGameandUI self (Variables|Default|GetLobby%20UI) "DoNotLock" true false)
    (CallFunction|ROSUpdatePlayerInfo)))

(fn ConstructionScript)