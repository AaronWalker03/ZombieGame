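; Lobby game mode that tracks connected player controllers and the BP_PlayerSlot actors they can occupy.
; BeginPlay orders the slots by numeric actor tags, while login and logout update the controller list.
; Both connection events then run a polling wait until the slots are ready.
; UpdatePlayerSlots calls AddPlayer on the first free slot for each unslotted controller, but no graph here calls it.
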(event EventBeginPlay
  (CallFunction|SetPlayerSlots))

(event EventOnLogout
  (params (ExitingController :type Controller%20Object%20Reference))
  (bind _asplayer_controller (Utilities|Casting|CastToPlayerController ExitingController))
  (Utilities|Array|RemoveItem (Variables|Default|GetPlayerControllers) _asplayer_controller)
  (Utilities|PlayerSlotsSet))

(event EventPostLogin
  (params (NewPlayer :type Player%20Controller%20Object%20Reference))
  (Utilities|Array|Add (Variables|Default|GetPlayerControllers) NewPlayer)
  (Utilities|PlayerSlotsSet))

(fn ConstructionScript)

(fn SetPlayerSlots
  (bind _outactors (Actor|GetAllActorsOfClass "/Game/Lobby/BP_PlayerSlot.BP_PlayerSlot_C"))
  (for _index (range 0 (Utilities|Array|LastIndex _outactors))
    (bind _outactors_2 (Actor|GetAllActorsOfClasswithTag "/Game/Lobby/BP_PlayerSlot.BP_PlayerSlot_C" (Utilities|String|StringToName (Utilities|String|ToString(Integer) _index))))
    (Utilities|Array|Add (Variables|Default|GetPlayerSlots) (Utilities|Array|Get(acopy) _outactors_2)))
  (Variables|Default|SetslotsSet true))

(fn UpdatePlayerSlots
  ;[0.15 0.15 0.15 0.5] Check if player controller is already added
  (for _array_element (Variables|Default|GetPlayerControllers)
    (LocalVariables|SetPlayer%20Controllers%20Added false)
    (bind _array_element_2 (Utilities|Array|ForEachLoopwithBreak (Variables|Default|GetPlayerSlots) :!label _label)
      (:LoopBody
        (if (== (Variables|/Game/Lobby/BP_PlayerSlot.BP_PlayerSlot_C|GetPlayerController _array_element_2) _array_element)
          (LocalVariables|SetPlayer%20Controllers%20Added true)
          (goto _label Break)))
      (:Completed
        (if (not (LocalVariables|GetPlayer%20Controllers%20Added))
          (bind _array_element_3 (Utilities|Array|ForEachLoopwithBreak (Variables|Default|GetPlayerSlots) :!label _label_2)
            (:LoopBody
              (Variables|/Game/Lobby/BP_PlayerSlot.BP_PlayerSlot_C|GetPlayerController _array_element_3
                (:then)
                (:else
                  (Default|AddPlayer _array_element_3)
                  (goto _label_2 Break))))))))))